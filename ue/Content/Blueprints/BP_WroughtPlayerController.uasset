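; Player controller for a first-person-style digging interface, which sends bite requests at the ground point under the camera's aim.
; Left click runs a long complex visibility trace from the camera and passes any hit location to RequestBite.
; Received bites update an assay panel widget created at BeginPlay.
; Keys set the depth tier and equip bare hand or sapling pick on WroughtSimSubsystem, with debug prints.
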(event Custom|OnBiteReceived_Event
  (params (Bite :type Wrought%20Bite%20Structure))
  (Default|UpdateAssay (Variables|Default|GetAssayPanel) Bite))

(event Custom|OnBiteReceived_Event_0
  (params (Bite :type Wrought%20Bite%20Structure)))

(event Custom|OnBiteReceived_Event_1
  (params (Bite :type Wrought%20Bite%20Structure)))

(event EventBeginPlay
  (Variables|Default|SetbShowMouseCursor false)
  (bind _returnvalue (UserInterface|CreateWidget "/Game/UI/WBP_AssayPanel.WBP_AssayPanel_C"))
  (Variables|Default|SetAssayPanel _returnvalue)
  (UserInterface|Viewport|AddtoViewport _returnvalue 0)
  (Input|SetInputModeGameOnly self false)
  (EventDispatchers|AssignOnBiteReceived (delegate Custom|OnBiteReceived_Event)))

(event EventTick
  (params (DeltaSeconds :type Float%20%28single-precision%29)))

(event Input|MouseEvents|LeftMouseButton
  (params (Key :type Key%20Structure))
  (bind _playercameramanager (Variables|Default|GetPlayerCameraManager))
  (bind _returnvalue (Camera|GetCameraLocation _playercameramanager))
  (:Pressed
    (bind (_outhit _returnvalue_2) (Collision|LineTraceByChannel _returnvalue (+ (* (Math|Vector|GetForwardVector (Camera|GetCameraRotation _playercameramanager)) "100000.0,100000.0,100000.0") _returnvalue) "TraceTypeQuery1" true 0 "None"))
    (if _returnvalue_2
      (Development|PrintString "TryBite: hit ground -> RequestBite")
      (Class|WroughtPlayerController|RequestBite (.Location (Collision|BreakHitResult _outhit))))))

(event Input|KeyboardEvents|1
  (params (Key :type Key%20Structure))
  (:Pressed
    (Variables|/Script/WroughtSim.WroughtSimSubsystem|SetSelectedTier (Subsystems|GetWroughtSimSubsystem) 0)
    (Development|PrintString "tier -> 0 (SURFACE)")))

(event Input|KeyboardEvents|2
  (params (Key :type Key%20Structure))
  (:Pressed
    (Variables|/Script/WroughtSim.WroughtSimSubsystem|SetSelectedTier (Subsystems|GetWroughtSimSubsystem) 1)
    (Development|PrintString "tier -> 1 (MIDDLE)")))

(event Input|KeyboardEvents|3
  (params (Key :type Key%20Structure))
  (:Pressed
    (Variables|/Script/WroughtSim.WroughtSimSubsystem|SetSelectedTier (Subsystems|GetWroughtSimSubsystem) 2)
    (Development|PrintString "tier -> 2 (DEEP)")))

(event Input|KeyboardEvents|F
  (params (Key :type Key%20Structure))
  (:Pressed
    (Class|WroughtSimSubsystem|EquipBareHand (Subsystems|GetWroughtSimSubsystem))
    (Development|PrintString "equipped: bare hand")))

(event Input|KeyboardEvents|R
  (params (Key :type Key%20Structure))
  (:Pressed
    (Class|WroughtSimSubsystem|EquipSaplingPick (Subsystems|GetWroughtSimSubsystem))
    (Development|PrintString "equipped: sapling pick")))

(fn ConstructionScript)